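; Enemy1BP is an AI enemy Blueprint that follows the closest player.
; Each Tick it updates animation and left/right rotation, selects the closest player and, when players are valid, moves toward them.
; It then checks whether it can act close to the player, but that branch is empty.
; The helper functions are defined outside this graph, and BeginPlay calls its parent while the parent Tick call is unconnected.
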(event EventBeginPlay
  (|CallParentFunction))

(event Collision|EventActorBeginOverlap
  (params (OtherActor :type Actor%20Object%20Reference))
  (|CallParentFunction OtherActor) ; This node is disabled and will not be called.\nDrag off pins to build functionality.
)

(event EventTick
  (params (DeltaSeconds :type Float%20%28single-precision%29))
  (CallFunction|UpdateAnimation)
  (CallFunction|SetAILeftRightRotation)
  (CallFunction|SetClosestPlayer)
  (bind _valid (CallFunction|PlayersValid))
  (if _valid
    (Utilities|FlowControl|Sequence
      (:then_0
        (CallFunction|MoveEnemytoPlayer 0.5))
      (:then_1
        (bind _doaction (CallFunction|CanDoActionClosetoPlayer))
        (if _doaction
          _)))))

(fn ConstructionScript
  (|CallParentFunction))