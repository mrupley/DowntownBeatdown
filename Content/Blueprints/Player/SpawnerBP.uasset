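; Spawner actor that creates and possesses a Paper2D player character, then handles its input and animation for side-view brawler movement and combat.
; Input events move the character and set punch, kick and special flags, with AcceptInput blocking most actions during attacks and landings.
; Tick picks flipbooks from those flags using DoOnce-and-Delay timed states, and flips facing via control rotation.
; Nested axis macros detect left/right double-taps, turning grounded punches into uppercuts.
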(event Custom|UpdateAnimation
  (bind _characterobject (Variables|Default|GetCharacterObject))
  (bind _characterobject_2 (Variables|Default|GetCharacterObject))
  (bind _returnvalue (Transformation|GetVelocity _characterobject))
  (bind _charactermovement (Variables|/Script/Engine.Character|GetCharacterMovement _characterobject))
  (bind _sprite (Variables|/Script/Paper2D.PaperCharacter|GetSprite _characterobject_2))
  (bind _returnvalue_2 (Math|Vector|VectorLength _returnvalue))
  (bind _returnvalue_3 (AI|Components|NavMovement|IsFalling _charactermovement))
  (bind _returnvalue_4 (> _returnvalue_2 0.0))
  ;[1 1 1] Handle Animation
  (if _returnvalue_3
    (Variables|Default|SetbIsAirborne true)
    (if (Variables|Default|GetbIsKicking)
      (Utilities|FlowControl|DoOnce false :!label _label
        (:Completed
          (Sprite|SetFlipbook _sprite "/Game/Art/Characters/Kunio/anim/anim_jumpkick1.anim_jumpkick1")
          (Utilities|FlowControl|Delay 0.4)
          (Variables|Default|SetbIsKicking false)
          (goto _label Reset)))
      (elif (Variables|Default|GetbIsPunching)
        (Utilities|FlowControl|DoOnce false :!label _label_2
          (:Completed
            (Sprite|SetFlipbook _sprite "/Game/Art/Characters/Kunio/anim/anim_punch1.anim_punch1")
            (Utilities|FlowControl|Delay 0.4)
            (Variables|Default|SetbIsPunching false)
            (goto _label_2 Reset)))
        (else
          (Sprite|SetFlipbook _sprite (select _returnvalue_3 "/Game/Art/Characters/Kunio/anim/anim_jump1.anim_jump1" "/Game/Art/Characters/Kunio/anim/aniim_idle1.aniim_idle1")))))
    (elif (Variables|Default|GetbIsAirborne)
      (Utilities|FlowControl|DoOnce false :!label _label_3
        (:Completed
          (Sprite|SetFlipbook _sprite "/Game/Art/Characters/Kunio/anim/anim_jumpland1.anim_jumpland1")
          (Variables|Default|SetbIsLanded true)
          (Utilities|FlowControl|Delay 0.4)
          (Variables|Default|SetbIsAirborne false)
          (Variables|Default|SetbIsLanded false)
          (goto _label_3 Reset)))
      (elif (Variables|Default|GetbIsKicking)
        (Utilities|FlowControl|DoOnce false :!label _label_4
          (:Completed
            (Sprite|SetFlipbook _sprite "/Game/Art/Characters/Kunio/anim/anim_kick1.anim_kick1")
            (Utilities|FlowControl|Delay 0.4)
            (Variables|Default|SetbIsKicking false)
            (goto _label_4 Reset)))
        (elif (Variables|Default|GetbIsPunching)
          (if (Variables|Default|GetbDoubleTapLeft)
            (Utilities|FlowControl|DoOnce false :!label _label_5
              (:Completed
                (Sprite|SetFlipbook _sprite "/Game/Art/Characters/Kunio/anim/anim_uppercut1.anim_uppercut1")
                (Utilities|FlowControl|Delay 0.4)
                (Variables|Default|SetbDoubleTapLeft false)
                (Variables|Default|SetbIsPunching false)
                (goto _label_5 Reset)))
            (elif (Variables|Default|GetbDoubleTapRight)
              (Utilities|FlowControl|DoOnce false :!label _label_6
                (:Completed
                  (Sprite|SetFlipbook _sprite "/Game/Art/Characters/Kunio/anim/anim_uppercut1.anim_uppercut1")
                  (Utilities|FlowControl|Delay 0.4)
                  (Variables|Default|SetbDoubleTapRight false)
                  (Variables|Default|SetbIsPunching false)
                  (goto _label_6 Reset)))
              (else
                (goto _label_2))))
          (elif (Variables|Default|GetbIsSpecial)
            (Sprite|SetFlipbook _sprite "/Game/Art/Characters/Kunio/anim/anim_shower.anim_shower")
            (else
              (Variables|Default|SetbIsWalking _returnvalue_4)
              (Sprite|SetFlipbook _sprite (select _returnvalue_4 "/Game/Art/Characters/Kunio/anim/anim_walk1.anim_walk1" "/Game/Art/Characters/Kunio/anim/aniim_idle1.aniim_idle1")))))))))

(event EventBeginPlay
  (bind _returnvalue (Transformation|GetActorTransform))
  ;[1 1 1] Create Player
  (bind _returnvalue_2 (Game|SpawnActorfromClass (Variables|Default|GetCharacter) (Math|Transform|MakeTransform (.location _returnvalue) (.rotation _returnvalue) (Math|Conversions|ToVector(Float) (Variables|Default|GetPlayer%20Size))) "Undefined" 0 0))
  (bind _aspaper_character (Utilities|Casting|CastToPaperCharacter _returnvalue_2))
  (bind _output_get (Variables|Default|SetCharacterObject _aspaper_character))
  (Pawn|Possess (Game|GetPlayerController 0) _output_get))

(event EventTick
  (params (DeltaSeconds :type Float%20%28single-precision%29))
  ;[1 1 1] Tick - Updates animation
  (CallFunction|UpdateAnimation)
  (Math|Float|CompareFloat (.X (Math|Vector|BreakVector (Variables|/Script/Engine.MovementComponent|GetVelocity (Pawn|GetMovementComponent (Variables|Default|GetCharacterObject))))) 0.0
    (:>
      (Pawn|SetControlRotation (Pawn|GetController (Variables|Default|GetCharacterObject)) (Math|Rotator|MakeRotator 0.0 0.0 0.0) :!label _label))
    (:==
      (if (Variables|Default|GetbisMovingRight)
        (goto _label)
        (else
          (Pawn|SetControlRotation (Pawn|GetController (Variables|Default|GetCharacterObject)) (Math|Rotator|MakeRotator 0.0 0.0 1.8e+02) :!label _label_2))))
    (:<
      (goto _label_2))))

(event Input|ActionEvents|InputActionKick
  (params (Key :type Key%20Structure :default "None"))
  ;[1 1 1] Combat State machine
  (:Pressed
    (bind _acceptinput (CallFunction|AcceptInput))
    (if _acceptinput
      (Variables|Default|SetbIsKicking true))))

(event Input|ActionEvents|InputActionJump
  (params (Key :type Key%20Structure :default "None"))
  (bind _characterobject (Variables|Default|GetCharacterObject))
  ;[1 1 1] Combat State machine
  (:Pressed
    (bind _acceptinput (CallFunction|AcceptInput))
    (if _acceptinput
      (Character|Jump _characterobject)))
  (:Released
    (Character|StopJumping _characterobject)))

(event Input|ActionEvents|InputActionPunch
  (params (Key :type Key%20Structure :default "None"))
  ;[1 1 1] Combat State machine
  (:Pressed
    (bind _acceptinput (CallFunction|AcceptInput))
    (if _acceptinput
      (Variables|Default|SetbIsPunching true))))

(event Input|ActionEvents|InputActionSpecial
  (params (Key :type Key%20Structure :default "None"))
  ;[1 1 1] Combat State machine
  (:Pressed
    (Variables|Default|SetbIsSpecial true))
  (:Released
    (Variables|Default|SetbIsSpecial false)))

(event Input|AxisEvents|InputAxisMoveUp
  (params (AxisValue :type Float%20%28single-precision%29))
  ;[1 1 1] Handle movement
  (bind _acceptinput (CallFunction|AcceptInput))
  (if _acceptinput
    (Pawn|Input|AddMovementInput (Variables|Default|GetCharacterObject) "0.000000,1.000000,0.000000" AxisValue false)))

(event Input|AxisEvents|InputAxisMoveRight
  (params (AxisValue :type Float%20%28single-precision%29))
  ;[1 1 1] Handle movement
  (bind _acceptinput (CallFunction|AcceptInput))
  (if _acceptinput
    (if (> AxisValue 0.0)
      (Variables|Default|SetbisMovingRight true)
      (Variables|Default|SetbDoubleTapLeft false)
      (elif (< AxisValue 0.0)
        (Variables|Default|SetbisMovingRight false)
        (Variables|Default|SetbDoubleTapRight false)))
    (Utilities|FlowControl|Sequence
      (:then_0
        (Pawn|Input|AddMovementInput (Variables|Default|GetCharacterObject) "1.000000, 0, 0" AxisValue false))
      (:then_1
        (Utilities|AxisDoubleTap AxisValue (Variables|Default|GetAxisThreshold) (Variables|Default|GetDoubleTapTimeout)
          (:Positive
            (Variables|Default|SetbDoubleTapRight true)
            ;[1 1 1] Tick - Updates animation
            (Development|PrintString "Right DT"))
          (:Negative
            (Variables|Default|SetbDoubleTapLeft true)
            (Development|PrintString "Left DT")))))))

(fn ConstructionScript)

(fn AcceptInput
  (if (Variables|Default|GetbIsPunching)
    _
    (elif (Variables|Default|GetbIsKicking)
      _
      (elif (Variables|Default|GetbIsLanded)
        _
        (else
          (return true)))))
  (return false))

(fn SetTap
  (bind _characterobject (Variables|Default|GetCharacterObject))
  (bind _returnvalue (Transformation|GetVelocity _characterobject))
  (bind _returnvalue_2 (Math|Vector|VectorLength _returnvalue))
  (if (not (< _returnvalue_2 0.0))
    (if (not (> _returnvalue_2 0.0))
      (if (== _returnvalue_2 0.0)
        (if (Variables|Default|GetbisMovingRight)
          _)))))