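; Shared orthographic camera that frames all players, tracking their sprites along the X axis.
; One frame after BeginPlay, to avoid a race on player references, it caches the GameMode's player list and becomes every PlayerController's view target.
; A looping timer centres it between the outermost players each update and sets ortho width to their clamped spread plus padding, leaving Y and Z unchanged.
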(event Custom|UpdateCamera
  (CallFunction|SetArmLength))

(event EventBeginPlay
  ;[1 1 1] Delay camera setup to next frame due to Player Reference race condition
  (Utilities|Time|SetTimerbyFunctionName 0 "UpdateCamera" 0.016 true)
  (Utilities|FlowControl|Delay 0.0)
  (CallFunction|ClassSetup))

(fn ConstructionScript)

(fn ClassSetup
  (bind _asgame_mode_bp (Utilities|Casting|CastToGameModeBP (Game|GetGameMode)))
  (bind _output_get (Variables|Default|SetBP%20Game%20Mode _asgame_mode_bp))
  (Variables|Default|SetPlayer%20Reference (Variables|/Game/Blueprints/Game/GameModeBP.GameModeBP_C|GetPlayers _output_get))
  (bind _outactors (Actor|GetAllActorsOfClass "/Script/Engine.PlayerController"))
  (Game|Player|SetViewTargetwithBlend _outactors self 0.0 "VTBlend_Linear" 0.0 false)
  (for (_array_element _array_index) (Variables|Default|GetPlayer%20Reference)
    (switch int _array_index
      (:0
        (Variables|Default|SetP1 _array_element))
      (:1
        (Variables|Default|SetP2 _array_element))
      (:2
        (Variables|Default|SetP3 _array_element))
      (:3
        (Variables|Default|SetP4 _array_element)))))

(fn SetArmLength
  (bind _positions (Variables|Default|Getpositions))
  (bind _mainspringcamera (Variables|Default|GetMainSpringCamera))
  (bind _returnvalue (Transformation|GetWorldLocation _mainspringcamera))
  (bind _maxvalue (Math|Float|MaxOfFloatArray _positions))
  (bind _minvalue (Math|Float|MinOfFloatArray _positions))
  (bind (_x _y _z) (Math|Vector|BreakVector _returnvalue))
  (for _array_element (Variables|Default|GetPlayer%20Reference)
    (Utilities|Array|AddUnique _positions (.X (Math|Vector|BreakVector (Transformation|GetWorldLocation (Variables|/Script/Paper2D.PaperCharacter|GetSprite _array_element))))))
  (Class|CameraComponent|SetOrthoWidth (Variables|Default|GetMainSpringCamera) (+ (Math|Float|Clamp(Float) (- _maxvalue _minvalue) (Variables|Default|GetMinArmLength) (Variables|Default|GetMaxArmLength)) (Variables|Default|GetCameraWidthPadding)))
  (Transformation|SetWorldLocation _mainspringcamera (Math|Vector|MakeVector (/ (+ _maxvalue _minvalue) 2.0) _y _z) false false)
  (Utilities|Array|Clear (Variables|Default|Getpositions)))