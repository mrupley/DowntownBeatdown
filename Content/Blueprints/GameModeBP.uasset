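; GameModeBP is a game mode that sets up local multiplayer pawns at BeginPlay.
; It caches all PlayerStart actors, then matches each player index up to MaxNumPlayers against PlayerStartTag.
; For each match it creates a local player, spawns a PlayerBP there, possesses it with that index's controller and records it in Players.
; GetPlayerArray returns the cached start points, not the spawned players.
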(event EventBeginPlay
  (CallFunction|GetPlayerStartPositions)
  (CallFunction|SpawnPlayers))

(fn ConstructionScript)

(fn GetPlayerStartPositions
  (bind _outactors (Actor|GetAllActorsOfClass "/Script/Engine.PlayerStart"))
  (Variables|Default|SetPlayerStartArray _outactors))

(fn SpawnPlayers
  (for _index (range 0 (- (Variables|Default|GetMaxNumPlayers) 1))
    (Variables|Default|Setindex _index)
    (for _array_element (Variables|Default|GetPlayerStartArray)
      (if (Utilities|Name|Equal(Name) (Variables|/Script/Engine.PlayerStart|GetPlayerStartTag _array_element) (Utilities|String|StringToName (Utilities|String|ToString(Integer) (Variables|Default|GetIndex))))
        (Class|GameplayStatics|CreatePlayer (Variables|Default|Getindex))
        (bind _returnvalue (Game|SpawnActorfromClass "/Game/Blueprints/Player/PlayerBP.PlayerBP_C" (Transformation|GetActorTransform _array_element) "Undefined" 0 0))
        (Pawn|Possess (Game|GetPlayerController (Variables|Default|Getindex)) _returnvalue)
        (Utilities|Array|AddUnique (Variables|Default|GetPlayers) _returnvalue)))))

(fn GetPlayerArray
  (return (Variables|Default|GetPlayerStartArray)))