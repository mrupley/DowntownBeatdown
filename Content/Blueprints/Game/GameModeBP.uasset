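; Game mode for a beat-synced game with local players and enemies, playing menu or gameplay music according to the Mode option.
; In Play mode it spawns and possesses pawns at index-tagged PlayerStarts and adds the HUD.
; A TimeSynth quarter-note quantization delegate drives beat tracking, feeding timing helpers and a DelayBeats macro that waits on beat boundaries.
; It also spawns and registers enemies, locks the camera while any exist, and applies the saved music setting.
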(event EventBeginPlay
  (bind _returnvalue (Game|GetGameMode))
  (bind _timesynth (Variables|Default|GetTimeSynth))
  (bind _optionsstring (Variables|/Script/Engine.GameModeBase|GetOptionsString _returnvalue))
  (CallFunction|CreateTimeSynth)
  (if (Utilities|Enum|Equal(Enum) (Class|GameplayStatics|ParseOption _optionsstring "Mode") "Play")
    (Variables|Default|SetMaxNumPlayers (Math|Conversions|ToInteger(Byte) (Class|GameplayStatics|ParseOption _optionsstring "NumPlayers")))
    (CallFunction|StartGamePlay)
    (Class|TimeSynthComponent|SetBPM _timesynth 1.2e+02)
    (Class|TimeSynthComponent|PlayClip _timesynth "/Game/Music/mega1_TimeSynthClip.mega1_TimeSynthClip" 0)
    (else
      (Class|TimeSynthComponent|SetBPM _timesynth 1.2e+02)
      (Class|TimeSynthComponent|PlayClip _timesynth "/Game/Music/mainmenu_1_TimeSynthClip.mainmenu_1_TimeSynthClip" 0)))
  (CallFunction|LoadSettings))

(fn ConstructionScript)

(fn GetPlayerStartPositions
  (bind _outactors (Actor|GetAllActorsOfClass "/Script/Engine.PlayerStart"))
  (Variables|Default|SetPlayerStartArray _outactors))

(fn SpawnPlayers
  (for _index (range 0 (- (Variables|Default|GetMaxNumPlayers) 1))
    (Variables|Default|Setindex _index)
    (for _array_element (Variables|Default|GetPlayerStartArray)
      (if (Utilities|Name|Equal(Name) (Variables|/Script/Engine.PlayerStart|GetPlayerStartTag _array_element) (Utilities|String|StringToName (Utilities|String|ToString(Integer) (Variables|Default|GetIndex))))
        (Class|GameplayStatics|CreatePlayer (Variables|Default|Getindex))
        (bind _returnvalue (Game|SpawnActorfromClass "/Game/Blueprints/Player/BasePlayer/BasePlayerBP.BasePlayerBP_C" (Transformation|GetActorTransform _array_element) "Undefined" 0 0))
        (Pawn|Possess (Game|GetPlayerController (Variables|Default|Getindex)) _returnvalue)
        (Utilities|Array|AddUnique (Variables|Default|GetPlayers) _returnvalue)))))

(fn GetPlayerArray
  (return (Variables|Default|GetPlayerStartArray)))

(fn StartGamePlay
  (CallFunction|GetPlayerStartPositions)
  (CallFunction|SpawnPlayers)
  (bind _returnvalue (UserInterface|CreateWidget "/Game/Blueprints/Widgets/HUD.HUD_C"))
  (UserInterface|Viewport|AddtoViewport _returnvalue 0))

(fn SetAudioBGMusic
  (params (NewParam :type Sound%20Base%20Object%20Reference))
  (bind _returnvalue (AddComponent|AddAudioComponent false))
  (Audio|Components|Audio|SetSound _returnvalue NewParam)
  (Variables|Default|SetBG_Music _returnvalue))

(fn OnBeat
  (params (QuantizationType :type ETimeSynthEventQuantization%20Enum :default "None") (NumBars :type Integer) (Beat :type Float%20%28single-precision%29))
  (bind _returnvalue (Math|Float|Truncate Beat))
  (bind _returnvalue_2 (* NumBars 4))
  ;[1 1 1] Current beat based on Quantization Type. Game Time comes from previous frame
  (Variables|Default|SetTimestampLastBeat (+ (Utilities|Time|GetGameTimeinSeconds) (Variables|Default|GetFrameDuration)))
  ;[1 1 1] Set total beats in current level (Beat sequence is 1,2,3,0 for OnBeat)
  (if (!= _returnvalue 0)
    (Variables|Default|SetBeatNumber (+ _returnvalue_2 _returnvalue))
    (else
      (Variables|Default|SetBeatNumber (+ _returnvalue_2 4)))))

(fn CreateTimeSynth
  ;[1 1 1] Create Time Synth
  (bind _returnvalue (AddComponent|AddTimeSynthComponent false))
  (bind _output_get (Variables|Default|SetTimeSynth _returnvalue))
  (CallFunction|GetBeatDuration)
  (Class|TimeSynthComponent|AddQuantizationEventDelegate _output_get "QuarterNote" (EventDispatchers|CreateEvent :!event OnBeat)))

(fn GetBeatDuration
  (return (/ 6e+01 (Math|Conversions|ToFloat(Integer) (Class|TimeSynthComponent|GetBPM (Variables|Default|GetTimeSynth))))))

(fn GetTimeSinceLastBeat
  ;[1 1 1] Time since last beat
  (return (- (Utilities|Time|GetGameTimeinSeconds) (Variables|Default|GetTimestampLastBeat))))

(fn GetBeatPercentage
  (bind _beatduration (CallFunction|GetBeatDuration))
  (bind _timesincelastbeat (CallFunction|GetTimeSinceLastBeat))
  (return (/ (+ _timesincelastbeat (Variables|Default|GetFrameDuration)) _beatduration)))

(fn SpawnEnemy
  (params (Class :type EnemyListEnum%20Enum :default "NewEnumerator1") (location :type Vector))
  (bind _returnvalue (Math|Conversions|ToTransform(Vector) location))
  (switch Utilities|FlowControl|Switch|SwitchonEnemyListEnum Class
    (:NewEnumerator1
      (bind _returnvalue_2 (Game|SpawnActorfromClass "/Game/Blueprints/Player/Enemies/BaseEnemy/BaseEnemyBP.BaseEnemyBP_C" _returnvalue "Undefined" 0 0))
      (LocalVariables|SetSpawnedEnemy _returnvalue_2))
    (:NewEnumerator0
      (bind _returnvalue_3 (Game|SpawnActorfromClass "/Game/Blueprints/Player/Enemies/Enemy1/Enemy1BP.Enemy1BP_C" _returnvalue "Undefined" 0 0))
      (LocalVariables|SetSpawnedEnemy _returnvalue_3))
    (:NewEnumerator2
      (bind _returnvalue_4 (Game|SpawnActorfromClass "/Game/Blueprints/Player/Enemies/Enemy2/Enemy2BP.Enemy2BP_C" _returnvalue "Undefined" 0 0))
      (LocalVariables|SetSpawnedEnemy _returnvalue_4)))
  (Utilities|Array|AddUnique (Variables|Default|GetEnemyArray) (LocalVariables|GetSpawnedEnemy))
  (Pawn|SpawnDefaultController (LocalVariables|GetSpawnedEnemy)))

(fn SetCameraLocked
  (Variables|Default|SetCameraLocked (> (Utilities|Array|Length (Variables|Default|GetEnemyArray)) 0)))

(fn GetDurationUntilNextBeat
  (bind _beatduration (CallFunction|GetBeatDuration))
  (bind _timesincelastbeat (CallFunction|GetTimeSinceLastBeat))
  (return (- _beatduration (+ _timesincelastbeat (Variables|Default|GetFrameDuration)))))

(fn GetDelayBeatDuration
  (params (Beats :type Integer))
  (bind _asgame_mode_bp (Utilities|Casting|CastToGameModeBP (Game|GetGameMode)))
  (bind _duration (CallFunction|GetDurationUntilNextBeat _asgame_mode_bp))
  (bind _beatduration (CallFunction|GetBeatDuration _asgame_mode_bp))
  (return (+ _duration (* Beats _beatduration))))

(fn LoadSettings
  (bind _timesynth (Variables|Default|GetTimeSynth))
  (bind _returnvalue (SaveGame|DoesSaveGameExist "Options"))
  (if _returnvalue
    (bind _returnvalue_2 (SaveGame|LoadGamefromSlot "Options"))
    (bind _assave_options (Utilities|Casting|CastToSaveOptions _returnvalue_2))
    (if (Variables|/Game/Blueprints/Menu/SaveOptions.SaveOptions_C|GetMusicOn _assave_options)
      (Audio|Components|Audio|SetVolumeMultiplier _timesynth 1.0 :!class /Script/AudioMixer.SynthComponent)
      (else
        (Audio|Components|Audio|SetVolumeMultiplier _timesynth 0.0 :!class /Script/AudioMixer.SynthComponent)))))